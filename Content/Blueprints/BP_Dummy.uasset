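; BP_Dummy is a target dummy that can be stealth-assassinated from behind.
; An overlap radius shows an assassinate prompt widget while BP_ThirdPersonCharacter is inside, and Tick turns the widget toward the camera.
; StealthBackAssassin plays the paired knife victim montage, triggers a delayed physics ragdoll, hides the prompt, and returns the AssassinRef location and dummy rotation as the attacker's alignment reference.
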(event `self.ReceiveTick`
  (params (DeltaSeconds :type "Float (single-precision)"))
  (`SceneComponent.K2_SetWorldRotation` (`self.Assassinate Widget`) (`KismetMathLibrary.FindLookAtRotation` (`SceneComponent.K2_GetComponentLocation` (`self.Assassinate Widget`)) (`SceneComponent.K2_GetComponentLocation` (`PlayerCameraManager.TransformComponent` (`GameplayStatics.GetPlayerCameraManager` 0)))) false false))

(event `Ragdoll`
  ;[1 1 1] Ragdoll
  (`KismetSystemLibrary.Delay` 2.5)
  (`PrimitiveComponent.SetSimulatePhysics` (`self.Mesh`) true))

(event `self.Assassination Radius.OnComponentBeginOverlap`
  (params (OverlappedComponent :type "PrimitiveComponent Object Reference") (OtherActor :type "Actor Object Reference") (OtherComp :type "PrimitiveComponent Object Reference") (OtherBodyIndex :type Integer) (bFromSweep :type Boolean) (SweepResult :type "HitResult Structure (by ref)"))
  (cast `/Game/ThirdPerson/Blueprints/BP_ThirdPersonCharacter` OtherActor)
  (`SceneComponent.SetVisibility` (`self.Assassinate Widget`) true false))

(event `self.Assassination Radius.OnComponentEndOverlap`
  (params (OverlappedComponent :type "PrimitiveComponent Object Reference") (OtherActor :type "Actor Object Reference") (OtherComp :type "PrimitiveComponent Object Reference") (OtherBodyIndex :type Integer))
  (cast `/Game/ThirdPerson/Blueprints/BP_ThirdPersonCharacter` OtherActor)
  (`SceneComponent.SetVisibility` (`self.Assassinate Widget`) false false))

(fn `Stealth Back Assassin`
  (returns (`REF Location` :type "Vector Structure") (`Assassin Rotation` :type "Rotator Structure"))
  (`self.PlayAnimMontage` "/Game/Characters/RPG_Character/Animations/Assassinations/Paired_Knife_Stealth_KidneyAndNeck_Vic_Montage.Paired_Knife_Stealth_KidneyAndNeck_Vic_Montage")
  (`self.Ragdoll`)
  (`SceneComponent.SetVisibility` (`self.Assassinate Widget`) false false)
  (return (`SceneComponent.K2_GetComponentLocation` (`self.Assassin Ref`)) (`self.K2_GetActorRotation`)))

(fn `UserConstructionScript`)